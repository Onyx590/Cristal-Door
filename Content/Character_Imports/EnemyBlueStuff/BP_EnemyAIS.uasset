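; Enemy AI character that chases the player once its pawn sensing sees a pawn and plays a montage on arrival.
; Tick halts its movement until that first sighting, which sets a seen flag that is never effectively cleared.
; Each sighting re-arms the attack flag and issues AI MoveTo toward player 0.
; Arrival calls PlayAnimMontage with no montage shown, delaying re-arming by its returned length; no damage is applied here.
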(event OnSeePawn(PawnSensing)
  (params (Pawn :type Pawn%20Object%20Reference))
  (Variables|Default|SetIsSeenPlayer true)
  (CallFunction|FollowPlayer))

(event Custom|Follow%20Player
  (Variables|Default|SetCanAttack true)
  (if (Variables|Default|GetIsSeenPlayer)
    (AI|AIMoveTo self "0, 0, 0" (Game|GetPlayerCharacter 0) 7e+01 false
      (:OnSuccess
        (if (Variables|Default|GetCanAttack)
          (Variables|Default|SetCanAttack false)
          (bind _returnvalue (Animation|PlayAnimMontage 0 1.0 "None"))
          (Utilities|FlowControl|Delay _returnvalue)
          (Variables|Default|SetCanAttack true))))
    (else
      (Variables|Default|SetIsSeenPlayer false))))

(event EventBeginPlay)

(event Collision|EventActorBeginOverlap
  (params (OtherActor :type Actor%20Object%20Reference)))

(event EventTick
  (params (DeltaSeconds :type Float%20%28single-precision%29))
  (if (not (Variables|Default|GetIsSeenPlayer))
    (Components|Movement|StopMovementImmediately (Variables|Character|GetCharacterMovement))))

(fn ConstructionScript)